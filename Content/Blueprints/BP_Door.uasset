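; BP_Door is a locked door that the player opens by spending a key.
; When a BP_ThirdPersonCharacterCustom overlaps its box trigger while still locked, it checks that character's KeyCount.
; With a key, it decrements the count, plays an open sound, sets DoorUnlocked and destroys the door mesh component.
; Without one, it prints a taunting on-screen message and plays a locked sound.
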(event OnComponentBeginOverlap(Boxcollision)
  (params (OverlappedComponent :type Primitive%20Component%20Object%20Reference) (OtherActor :type Actor%20Object%20Reference) (OtherComp :type Primitive%20Component%20Object%20Reference) (OtherBodyIndex :type Integer) (bFromSweep :type Boolean) (SweepResult :type Hit%20Result%20Structure%20%28by%20ref%29))
  (bind _asbp_third_person_character_custom (Utilities|Casting|CastToBP_ThirdPersonCharacterCustom OtherActor))
  (if (not (Variables|Default|GetDoorUnlocked))
    (if (> (Variables|/Game/Blueprints/BP_ThirdPersonCharacterCustom.BP_ThirdPersonCharacterCustom_C|GetKey%20Count _asbp_third_person_character_custom) 0) ; Like an If Statement
      (Variables|/Game/Blueprints/BP_ThirdPersonCharacterCustom.BP_ThirdPersonCharacterCustom_C|SetKey%20Count _asbp_third_person_character_custom (- (Variables|/Game/Blueprints/BP_ThirdPersonCharacterCustom.BP_ThirdPersonCharacterCustom_C|GetKey%20Count _asbp_third_person_character_custom) 1)) ; Remove a Key, then open door.
      (Audio|PlaySoundatLocation "/Game/Audio/Door_Open_Cue.Door_Open_Cue" (Transformation|GetWorldLocation (Variables|Default|GetDefaultSceneRoot)) "0, 0, 0" 1.0 1.0 0.0 0 0 0 0)
      (Variables|Default|SetDoorUnlocked true)
      (Components|DestroyComponent (Variables|Default|GetSM_Door))
      (else
        (Development|PrintString "Where do you think you're going? Get back in the kitchen!" true true "(R=0.479167,G=0.051103,B=0.000000,A=1.000000)" 5.0)
        (Audio|PlaySoundatLocation "/Game/Audio/Door_Locked_Cue.Door_Locked_Cue" (Transformation|GetWorldLocation (Variables|Default|GetDefaultSceneRoot)) "0, 0, 0" 1.0 1.0 0.0 0 0 0 0)))))

(event EventBeginPlay)

(event Collision|EventActorBeginOverlap
  (params (OtherActor :type Actor%20Object%20Reference)))

(event EventTick
  (params (DeltaSeconds :type Float%20%28single-precision%29)))

(fn ConstructionScript)