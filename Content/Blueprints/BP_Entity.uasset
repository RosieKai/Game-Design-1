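; Entity Blueprint that emits crowd murmurs, voices and whispers from its Head component as ambient audio.
; An entity flagged StartingBoi plays a pre-movie cinema chatter cue once, then fades it out; others start a self-recalling PlayAudio loop after a delay.
; Each pass picks a random cue and either plays it occasionally, with random delay and fade-out, or waits and retries.
; CeaseAudio clears Playable to end the loop, stopping the sound if IsPlaying.
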(event Custom|SwitchAudio
  (switch int (Math|Random|RandomIntegerinRange 0 4)
    (:Default
      (Development|PrintString "Fail"))
    (:0
      (Variables|Default|SetStage1 "/Game/Audio/Whispers/FourVoices1_Cue.FourVoices1_Cue"))
    (:1
      (Variables|Default|SetStage1 "/Game/Audio/Whispers/FourVoices2_Cue.FourVoices2_Cue"))
    (:2
      (Variables|Default|SetStage1 "/Game/Audio/Whispers/IndistinceWhispers_Cue.IndistinceWhispers_Cue"))
    (:3
      (Variables|Default|SetStage1 "/Game/Audio/Whispers/Murmullos_Cue.Murmullos_Cue"))
    (:4
      (Variables|Default|SetStage1 "/Game/Audio/Whispers/Murmurs_Cue.Murmurs_Cue"))))

(event Custom|PlayAudio
  (if (Variables|Default|GetPlayable)
    (CallFunction|SwitchAudio)
    (switch int (Math|Random|RandomIntegerinRange 0 5)
      (:Default
        (Development|PrintString "Fail"))
      (:0
        (Variables|Default|SetisPlaying true)
        (Utilities|FlowControl|Delay (Math|Random|RandomFloatinRange 1.0 15.0))
        (Development|PrintString "PLaying Audio")
        (bind _returnvalue (Audio|SpawnSoundAttached (Variables|Default|GetStage1) (Variables|Default|GetHead) "None" "0, 0, 0" "0, 0, 0" "KeepRelativeOffset" false 1.0 1.0 0.0 0 0))
        (Utilities|FlowControl|Delay 2e+01)
        (Audio|Components|Audio|FadeOut _returnvalue 5.0 0.0 "Linear" :!class /Script/Engine.AudioComponent)
        (CallFunction|PlayAudio)
        (Variables|Default|SetisPlaying false))
      (:1
        (Variables|Default|SetisPlaying false :!label _label)
        (Utilities|FlowControl|Delay 5.0)
        (CallFunction|PlayAudio))
      (:2
        (goto _label))
      (:3
        (goto _label))
      (:4
        (goto _label))
      (:5
        (goto _label)))))

(event Custom|CeaseAudio
  (if (Variables|Default|GetisPlaying)
    (Audio|Components|Audio|Stop (stale Custom|PlayAudio _returnvalue))
    (Variables|Default|SetPlayable false)
    (else
      (Variables|Default|SetPlayable false))))

(event EventBeginPlay
  (if (Variables|Default|GetStartingBoi)
    (bind _returnvalue (Audio|SpawnSoundAttached "/Game/Audio/Whispers/people-talking-in-cinema-before-movie-starts-65662_Cue.people-talking-in-cinema-before-movie-starts-65662_Cue" (Variables|Default|GetHead) "None" "0, 0, 0" "0, 0, 0" "KeepRelativeOffset" false 1.0 1.0 0.0 0 0))
    (Utilities|FlowControl|Delay 2e+01)
    (Audio|Components|Audio|FadeOut _returnvalue 5.0 0.0 "Linear" :!class /Script/Engine.AudioComponent)
    (else
      (Utilities|FlowControl|Delay 1e+01)
      (CallFunction|PlayAudio))))

(fn ConstructionScript)