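; BP_Oven is an oven that takes an uncooked pizza from the player character and cooks it.
; When an actor overlaps CookBox, it casts to BP_ThirdPersonCharacterCustom and, if an uncooked pizza is held, calls Cook with OvenBase and empties the character's hands.
; A GotPizza flag blocks further pizzas until a fixed delay clears it, with debug strings reporting busy and ready states.
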(event OnComponentBeginOverlap(CookBox)
  (params (OverlappedComponent :type Primitive%20Component%20Object%20Reference) (OtherActor :type Actor%20Object%20Reference) (OtherComp :type Primitive%20Component%20Object%20Reference) (OtherBodyIndex :type Integer) (bFromSweep :type Boolean) (SweepResult :type Hit%20Result%20Structure%20%28by%20ref%29))
  (if (Variables|Default|GetGotPizza)
    (Development|PrintString "there's a pizza here already")
    (else
      (bind _asbp_third_person_character_custom (Utilities|Casting|CastToBP_ThirdPersonCharacterCustom OtherActor))
      (switch Utilities|FlowControl|Switch|SwitchonE_PizzaItem (Variables|/Game/Blueprints/BP_ThirdPersonCharacterCustom.BP_ThirdPersonCharacterCustom_C|GetItemHeld _asbp_third_person_character_custom)
        (:NewEnumerator5
          (Default|Cook (Variables|/Game/Blueprints/BP_ThirdPersonCharacterCustom.BP_ThirdPersonCharacterCustom_C|GetHeldItem _asbp_third_person_character_custom) (Variables|Default|GetOvenBase))
          (Variables|/Game/Blueprints/BP_ThirdPersonCharacterCustom.BP_ThirdPersonCharacterCustom_C|SetHeldItem _asbp_third_person_character_custom 0)
          (Variables|/Game/Blueprints/BP_ThirdPersonCharacterCustom.BP_ThirdPersonCharacterCustom_C|SetItemHeld _asbp_third_person_character_custom "NewEnumerator4")
          (Variables|Default|SetGotPizza true)
          (Utilities|FlowControl|Delay 3e+01)
          (Variables|Default|SetGotPizza false)
          (Development|PrintString "Oven is ready"))))))

(event EventBeginPlay
  (Variables|Default|SetGotPizza false))

(fn ConstructionScript)