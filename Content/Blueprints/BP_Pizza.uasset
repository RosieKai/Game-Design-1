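; BP_Pizza is a pizza item that players carry, bake, eat or serve, attaching to the hand or oven socket.
; Bake re-calls itself after a delay, advancing CookProg from raw to cooked to burnt; InOven gates only the burnt visuals, not the counter.
; Overlap offers cooked or burnt pizza to the character for pickup, clearing InOven.
; Eating prints a state-based message and destroys it, with health still TODO; serving destroys it silently.
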(event OnComponentBeginOverlap(PickupTrigger)
  (params (OverlappedComponent :type Primitive%20Component%20Object%20Reference) (OtherActor :type Actor%20Object%20Reference) (OtherComp :type Primitive%20Component%20Object%20Reference) (OtherBodyIndex :type Integer) (bFromSweep :type Boolean) (SweepResult :type Hit%20Result%20Structure%20%28by%20ref%29))
  (bind _self self)
  (switch int (Variables|Default|GetCookProg)
    (:Default
      (Development|PrintString "Huh???"))
    (:1
      (bind _asbp_third_person_character_custom (Utilities|Casting|CastToBP_ThirdPersonCharacterCustom OtherActor))
      (Default|TrytoPickUp _asbp_third_person_character_custom _self "NewEnumerator6")
      (Variables|Default|SetInOven false))
    (:2
      (bind _asbp_third_person_character_custom_2 (Utilities|Casting|CastToBP_ThirdPersonCharacterCustom OtherActor))
      (Default|TrytoPickUp _asbp_third_person_character_custom_2 _self "NewEnumerator7")
      (Variables|Default|SetInOven false))))

(event Custom|Bake
  (bind _pizzadough (Variables|Default|GetPizzaDough))
  (Utilities|FlowControl|Delay 6.0)
  (bind _output_get (Variables|Default|SetCookProg (+ (Variables|Default|GetCookProg) 1)))
  (if (<= _output_get 1)
    (Rendering|Material|SetMaterial _pizzadough 0 "/Game/Materials/MI_CookDough.MI_CookDough")
    (Development|PrintString "~Ding~" true true "(R=0.000000,G=0.000000,B=0.000000,A=1.000000)")
    (CallFunction|Bake)
    (elif (Variables|Default|GetInOven)
      (Development|PrintString "~BEEP BEEP BEEP~" true true "(R=0.000000,G=0.000000,B=0.000000,A=1.000000)")
      (Rendering|Material|SetMaterial _pizzadough 0 "/Game/Materials/MI_BurnDough.MI_BurnDough"))))

(event EventCook
  (params (Placement :type Static%20Mesh%20Component%20Object%20Reference))
  (bind _pizzadough (Variables|Default|GetPizzaDough))
  (Transformation|AttachComponentToComponent _pizzadough Placement "Base" "SnapToTarget" "KeepRelative" "KeepRelative" false)
  (Transformation|SetWorldLocation _pizzadough (+ (Transformation|GetWorldLocation _pizzadough) "0.000000,0.000000,50.000000") false true)
  (Collision|SetCollisionEnabled _pizzadough "NoCollision") ; Collide with the ground please
  (Variables|Default|SetInOven true)
  (CallFunction|Bake))

(event EventBeginPlay
  (Variables|Default|SetCookProg 0)
  (Rendering|Material|SetMaterial (Variables|Default|GetPizzaDough) 0 "/Game/Materials/MI_Dough.MI_Dough")
  (Variables|Default|SetInOven false))

(event EventPickup
  (params (ParentMesh :type Skeletal%20Mesh%20Component%20Object%20Reference))
  (bind _pizzadough (Variables|Default|GetPizzaDough))
  (Transformation|AttachComponentToComponent _pizzadough ParentMesh "hand_r" "SnapToTarget" "KeepRelative" "KeepRelative" true)
  (Collision|SetCollisionEnabled _pizzadough "NoCollision") ; Collide with the ground please
)

(event EventServe
  (params (Ref_ThirdPerson :type BP%20Third%20Person%20Character%20Custom%20Object%20Reference))
  (Variables|/Game/Blueprints/BP_ThirdPersonCharacterCustom.BP_ThirdPersonCharacterCustom_C|SetHeldItem Ref_ThirdPerson 0) ; Set the player's held item to nothing
  (Actor|DestroyActor) ; destroy this item
)

(event EventPrimaryAction
  (params (ref_thirdPersonCharCustom :type BP%20Third%20Person%20Character%20Custom%20Object%20Reference))
  (Variables|/Game/Blueprints/BP_ThirdPersonCharacterCustom.BP_ThirdPersonCharacterCustom_C|SetHeldItem ref_thirdPersonCharCustom 0) ; Set the player's held item to nothing
  (Rendering|Material|SetMaterial (Variables|Default|GetPizzaDough) 0 "/Game/Materials/MI_Dough.MI_Dough")
  (switch int (Variables|Default|GetCookProg)
    (:Default
      (Development|PrintString "Huh???"))
    (:0
      (Development|PrintString "But... It's raw... okay... if you're sure.... You eated it." true true "(R=0.232018,G=0.316761,B=0.360417,A=1.000000)") ; TODO: Implement a health system.
      (Variables|Default|SetCookProg 0)
      (Actor|DestroyActor) ; destroy this item
    )
    (:1
      (Development|PrintString "Yummy Pizza!" true true "(R=0.232018,G=0.316761,B=0.360417,A=1.000000)") ; TODO: Implement a health system.
      (Variables|Default|SetCookProg 0)
      (Actor|DestroyActor) ; destroy this item
    )
    (:2
      (Development|PrintString "You eated a yucky, burnt pizza :(" true true "(R=0.232018,G=0.316761,B=0.360417,A=1.000000)") ; TODO: Implement a health system.
      (Variables|Default|SetCookProg 0)
      (Actor|DestroyActor) ; destroy this item
    )))

(fn ConstructionScript)