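; BP_SpawnCheese is a pickup point that hands cheese to the player character.
; Overlapping its Box calls TryToPickUp on the custom third-person character, passing itself.
; Its Pickup event spawns a new BP_Cheese at the Sphere's location, snaps it to the hand_r socket of the supplied mesh and disables collision on its CHEESE component.
; The spawner is not destroyed by the pickup.
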(event OnComponentBeginOverlap(Box)
  (params (OverlappedComponent :type Primitive%20Component%20Object%20Reference) (OtherActor :type Actor%20Object%20Reference) (OtherComp :type Primitive%20Component%20Object%20Reference) (OtherBodyIndex :type Integer) (bFromSweep :type Boolean) (SweepResult :type Hit%20Result%20Structure%20%28by%20ref%29))
  (bind _asbp_third_person_character_custom (Utilities|Casting|CastToBP_ThirdPersonCharacterCustom OtherActor))
  (Default|TrytoPickUp _asbp_third_person_character_custom self))

(event EventPickup
  (params (ParentMesh :type Skeletal%20Mesh%20Component%20Object%20Reference))
  (bind _returnvalue (Game|SpawnActorfromClass "/Game/Blueprints/BP_Cheese.BP_Cheese_C" (Math|Transform|MakeTransform (Transformation|GetWorldLocation (Variables|Default|GetSphere))) "Undefined" "MultiplyWithRoot" 0 0))
  (Transformation|AttachComponentToComponent (Variables|/Script/Engine.Actor|GetRootComponent _returnvalue) ParentMesh "hand_r" "SnapToTarget" "KeepRelative" "KeepRelative" true)
  (Collision|SetCollisionEnabled (Variables|/Game/Blueprints/BP_Cheese.BP_Cheese_C|GetCHEESE _returnvalue) "NoCollision") ; Collide with the ground please
)

(fn ConstructionScript)