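; Spawner actor that creates one random shape actor (circle, triangle or diamond) at its Emitter when play begins.
; BeginPlay hides the R component and rolls 0 to 3 to choose the class, so a 3 prints an error and spawns nothing.
; SpawnThing spawns the class and, if it casts to BP_CanOfBeans, gives its Lid a random material from MatArray.
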(event Custom|SpawnThing
  (params (The%20Thing :type Actor%20Class%20Reference))
  (bind _returnvalue (Game|SpawnActorfromClass The%20Thing (Transformation|GetWorldTransform (Variables|Default|GetEmitter)) "Undefined" "MultiplyWithRoot" 0 0))
  (bind _asbp_can_of_beans (Utilities|Casting|CastToBP_CanOfBeans _returnvalue))
  (Rendering|Material|SetMaterial (Variables|/Game/Blueprints/BP_CanOfBeans.BP_CanOfBeans_C|GetLid _asbp_can_of_beans) 0 (.OutItem (Utilities|Array|Random (Variables|Default|GetMatArray)))))

(event EventBeginPlay
  (Rendering|SetVisibility (Variables|Default|Getr) false false)
  (switch int (Math|Random|RandomIntegerinRange 0 3)
    (:Default
      (Development|PrintString "Error"))
    (:0
      (Variables|Default|SetThe%20Thing "/Game/Blueprints/BP_Circle.BP_Circle_C")
      (CallFunction|SpawnThing (stale _output_get) :!label _label))
    (:1
      (Variables|Default|SetThe%20Thing "/Game/Blueprints/BP_Triangle.BP_Triangle_C")
      (goto _label))
    (:2
      (bind _output_get (Variables|Default|SetThe%20Thing "/Game/Blueprints/BP_Diamond.BP_Diamond_C"))
      (goto _label))))

(fn ConstructionScript)