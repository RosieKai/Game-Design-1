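; Cube Blueprint that switches its static mesh from a wall material to an opacity-animated material shortly after play begins.
; On BeginPlay it applies MI_Walls, waits a few seconds, then creates and assigns a dynamic instance of OTest.
; The Fade timeline then plays from the start, feeding its track value into the instance's Opacity parameter on each update.
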(event EventBeginPlay
  (Rendering|Material|SetMaterial (Variables|Debug|GetStaticMeshComponent) 0 "/Game/Materials/MI_Walls.MI_Walls")
  (Utilities|FlowControl|Delay 5.0)
  (bind _returnvalue (Rendering|Material|CreateDynamicMaterialInstance "/Game/Materials/OTest.OTest" "None" "None" :!class /Script/Engine.KismetMaterialLibrary))
  (Variables|Default|SetMID _returnvalue)
  (Rendering|Material|SetMaterial (Variables|Debug|GetStaticMeshComponent) 0 (Variables|Default|GetMID))
  (Components|Timeline|PlayfromStart (Variables|Default|GetFade)))

(fn ConstructionScript)